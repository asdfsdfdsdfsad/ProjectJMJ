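; BP_AIPerson is an AI character Blueprint that displays its health on a widget and seeds its AI blackboard.
; On BeginPlay it binds to the AttributeComponent's health-changed event and writes a fixed AttackRange value into the AI controller's blackboard.
; Health changes pass the Damage value to the WB_AIHealth widget held by its widget component.
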(event `self.ReceiveBeginPlay`
  (add `AttributeComponent.OnHealthChanged` (`self.AttributeComponent`) (delegate `SetHealth`))
  (`BlackboardComponent.SetValueAsFloat` (`AIBlueprintHelperLibrary.GetBlackboard` (`AIBlueprintHelperLibrary.GetAIController` (`self.GetController`))) (`self.AttackRange`) 200.0))

(event `SetHealth`
  (params (InstigatorActor :type "Actor Object Reference") (OwningComp :type "AttributeComponent Object Reference") (Damage :type "Float (single-precision)") (Delta :type "Float (single-precision)") (HitLocation :type "Vector Structure"))
  (bind _aswb_aihealth (cast `/Game/UI/WB_AIHealth` (`WidgetComponent.GetWidget` (`self.Widget`))))
  (`/Game/UI/WB_AIHealth.Set Health` _aswb_aihealth Damage))

(event `self.ReceiveTick`
  (params (DeltaSeconds :type "Float (single-precision)")))

(fn `UserConstructionScript`)