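; BP_Ability1 is an ability actor with a Niagara effect (NIAbility1) and a ProjectileMovement component.
; SetNiagara passes a rotator to the effect's "Rotation" variable as a roll, pitch, yaw vector, and SetActivates1 activates projectile movement with a reset.
; The event graph does nothing at runtime, holding only empty events and disconnected attach, delayed upward-move and debug print nodes.
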(event `self.ReceiveBeginPlay`)

(event `self.ReceiveTick`
  (params (DeltaSeconds :type "Float (single-precision)")))

(fn `Set Activates 1`
  (`ActorComponent.SetActive` (`self.ProjectileMovement`) true true))

(fn `SetNiagara`
  (params (Rotation :type "Rotator Structure"))
  (`NiagaraComponent.SetVariableVec3` (`self.NI_Ability1`) "Rotation" (`KismetMathLibrary.MakeVector` (.roll Rotation) (.pitch Rotation) (.yaw Rotation))))

(fn `UserConstructionScript`)