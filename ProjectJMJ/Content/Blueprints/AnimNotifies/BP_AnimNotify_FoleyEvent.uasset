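; BP_AnimNotify_FoleyEvent is an anim notify for tag-driven foley sounds, named in the timeline after its event tag.
; Its logic gets a foley audio bank, gates Run events on the owner's footstep check, and plays the sound at the mesh.
; A console variable enables debug spheres at the mesh or chosen foot.
; As shown, both ReceivedNotify and GetAudioBank entries are empty, leaving playback logic unconnected.
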(fn `GetAudioBank`
  (params (MeshComponent :type "SkeletalMeshComponent Object Reference"))
  (returns (Bank :type "Object Object Reference") (CanPlaySound :type Boolean))
  (locals (MeshCompo :type "SkeletalMeshComponent Object Reference")))

(fn `GetNotifyName`
  (returns (ReturnValue :type String))
  (return (`KismetTextLibrary.Conv_TextToString` (`|FormatText` "FoleyEvent: {Type}" (`.RightS` (`KismetStringLibrary.Split` (`BlueprintGameplayTagLibrary.GetDebugStringFromGameplayTag` (`self.Event`)) "." "IgnoreCase" "FromEnd"))))))

(fn `Received_Notify`
  (params (MeshComp :type "SkeletalMeshComponent Object Reference") (Animation :type "AnimSequenceBase Object Reference") (EventReference :type "AnimNotifyEventReference Structure (by ref)"))
  (returns (ReturnValue :type Boolean))
  (locals (MeshComponent :type "SkeletalMeshComponent Object Reference")))